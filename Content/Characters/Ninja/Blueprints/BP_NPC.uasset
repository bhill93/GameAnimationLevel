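; NPC that plays voiced dialogue from DT_NPCDialogue when a SandboxCharacter_CMC1 enters its sphere.
; Overlap registers the NPC on the player and shows the dialogue widget, and leaving removes both.
; NextLine walks rows from IndexStart, playing audio and tilting and justifying text by speaker, until an empty line or table end resets it.
; An older DialogueLines array path remains unconnected.
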(event `self.ReceiveBeginPlay`
  (bind _returnvalue (`|CreateWidget` "/Game/Widgets/W_NPCDialogue.W_NPCDialogue_C"))
  (set `self.W_Dialogue` _returnvalue)
  (set `self.NextLineIndex` (`self.IndexStart`)))

(event `self.Sphere.OnComponentBeginOverlap`
  (params (OverlappedComponent :type "PrimitiveComponent Object Reference") (OtherActor :type "Actor Object Reference") (OtherComp :type "PrimitiveComponent Object Reference") (OtherBodyIndex :type Integer) (bFromSweep :type Boolean) (SweepResult :type "HitResult Structure (by ref)"))
  (bind _assandbox_character_cmc1 (cast `/Game/SandboxCharacter_CMC1` OtherActor))
  (bind _output_get (set `self.Player` _assandbox_character_cmc1))
  (set `/Game/SandboxCharacter_CMC1.NPC` self _output_get)
  (`UserWidget.AddToViewport` (`self.W_Dialogue`) 0)
  (`self.next Line`))

(event `self.Sphere.OnComponentEndOverlap`
  (params (OverlappedComponent :type "PrimitiveComponent Object Reference") (OtherActor :type "Actor Object Reference") (OtherComp :type "PrimitiveComponent Object Reference") (OtherBodyIndex :type Integer))
  (cast `/Game/SandboxCharacter_CMC1` OtherActor)
  (`self.End Dialogue`))

(event `End Dialogue`
  (set `/Game/SandboxCharacter_CMC1.NPC` null (`self.Player`))
  (set `self.Player` null)
  (`Widget.RemoveFromParent` (`self.W_Dialogue`))
  (set `self.NextLineIndex` (`self.IndexStart`)))

(event `Next Line`
  (bind _audiocomponent (`self.AudioComponent`))
  (bind _textblock_0 (`/Game/Widgets/W_NPCDialogue.TextBlock_0` (`self.W_Dialogue`)))
  (bind _outrownames (`DataTableFunctionLibrary.GetDataTableRowNames` "/Game/Blueprints/DT_NPCDialogue.DT_NPCDialogue"))
  (if (> (`self.NextLineIndex`) (`KismetArrayLibrary.Array_LastIndex` _outrownames))
    (`self.End Dialogue`)
    (else
      (bind _returnvalue (`|GetDataTableRow` "/Game/Blueprints/DT_NPCDialogue.DT_NPCDialogue" (`|GetArrayItem` _outrownames (`self.NextLineIndex`)))
        (:`then`
          (if (`KismetStringLibrary.EqualEqual_StrStr` (break `/Game/Blueprints/S_NPCDialogue` _returnvalue))
            (`self.End Dialogue`)
            (else
              (`TextBlock.SetText` (`/Game/Widgets/W_NPCDialogue.TextBlock_0` (`self.W_Dialogue`)) (`KismetTextLibrary.Conv_StringToText` (break `/Game/Blueprints/S_NPCDialogue` _returnvalue)))
              (`/Engine/EditorBlueprintResources/StandardMacros.IncrementInt` (`self.NextLineIndex`)
                (:`  `
                  (`AudioComponent.SetSound` _audiocomponent (`.VoicedLine_7_20F712D849CB125D2AF742BD3EC25FEB` (break `/Game/Blueprints/S_NPCDialogue` _returnvalue)))
                  (`AudioComponent.Play` _audiocomponent 0.0)
                  (switch `/Game/Blueprints/E_Speaker` (`.Speaker_8_B9E5F9D546BF860B7A1CDEA60DB6F9C8` (break `/Game/Blueprints/S_NPCDialogue` _returnvalue))
                    (:`NewEnumerator0`
                      (`Widget.SetRenderTransformAngle` _textblock_0 (`KismetMathLibrary.RandomFloatInRange` -5.5 -4.5))
                      (set `TextLayoutWidget.Justification` "Left" _textblock_0))
                    (:`NewEnumerator1`
                      (`Widget.SetRenderTransformAngle` _textblock_0 (`KismetMathLibrary.RandomFloatInRange` 4.5 5.5))
                      (set `TextLayoutWidget.Justification` "Right" _textblock_0))))))))))))

(fn `UserConstructionScript`)