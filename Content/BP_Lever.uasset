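; Lever actor that makes an overlapping Sandbox CMC character reach its right hand to the handle through IK.
; Sphere overlap caches the character's Anim Blueprint, sets the IK target to the handle's world location and plays a timeline that blends in the hand IK alpha.
; Once blended, a delayed self-calling event keeps refreshing the target during overlap, and leaving the sphere reverses the timeline.
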(event `self.SphereCollision.OnComponentBeginOverlap`
  (params (OverlappedComponent :type "PrimitiveComponent Object Reference") (OtherActor :type "Actor Object Reference") (OtherComp :type "PrimitiveComponent Object Reference") (OtherBodyIndex :type Integer) (bFromSweep :type Boolean) (SweepResult :type "HitResult Structure (by ref)"))
  (bind _assandbox_character_cmc1 (cast `/Game/SandboxCharacter_CMC1` OtherActor))
  (bind _assandbox_character_cmc_abp1 (cast `/Game/SandboxCharacter_CMC_ABP1` (`SkeletalMeshComponent.GetAnimInstance` (`Character.Mesh` _assandbox_character_cmc1))))
  (bind _output_get (set `self.AnimBP` _assandbox_character_cmc_abp1))
  (set `self.TouchingButton` true)
  (set `/Game/SandboxCharacter_CMC_ABP1.Right Hand IK Target` (`SceneComponent.K2_GetComponentLocation` (`self.Handle`)) _output_get)
  (bind (_direction _newtrack_0) (`Timeline|Timeline` :!via `PlayFromStart` :!label _label)
    (:`Update`
      (set `/Game/SandboxCharacter_CMC_ABP1.Right Hand IK Alpha` _newtrack_0 (`self.AnimBP`)))
    (:`Finished`
      (`self.UpdateHandPosition`))))

(event `self.SphereCollision.OnComponentEndOverlap`
  (params (OverlappedComponent :type "PrimitiveComponent Object Reference") (OtherActor :type "Actor Object Reference") (OtherComp :type "PrimitiveComponent Object Reference") (OtherBodyIndex :type Integer))
  (set `self.TouchingButton` false)
  (goto _label :!via `Reverse`))

(event `UpdateHandPosition`
  (if (`self.TouchingButton`)
    (bind _animbp (`self.AnimBP`)
      (:`then`
        (set `/Game/SandboxCharacter_CMC_ABP1.Right Hand IK Target` (`SceneComponent.K2_GetComponentLocation` (`self.Handle`)) _animbp)
        (`KismetSystemLibrary.Delay` 0.1)
        (`self.UpdateHandPosition`))
      (:`else`))))

(fn `UserConstructionScript`)